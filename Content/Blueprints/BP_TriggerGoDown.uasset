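; Trigger volume that sends a linked Elevator downward when the third-person player character leaves its box.
; On end overlap it compares the elevator's CurrentFloor to its own MyStep.
; An elevator at or below MyStep moves to the floor under MyStep, while one above moves to MyStep.
; Begin overlap only casts to the character and takes no action.
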(event `self.Box.OnComponentBeginOverlap`
  (params (OverlappedComponent :type "PrimitiveComponent Object Reference") (OtherActor :type "Actor Object Reference") (OtherComp :type "PrimitiveComponent Object Reference") (OtherBodyIndex :type Integer) (bFromSweep :type Boolean) (SweepResult :type "HitResult Structure (by ref)"))
  (cast `/Game/Blueprints/BP_ThirdPersonCharacter` OtherActor))

(event `self.Box.OnComponentEndOverlap`
  (params (OverlappedComponent :type "PrimitiveComponent Object Reference") (OtherActor :type "Actor Object Reference") (OtherComp :type "PrimitiveComponent Object Reference") (OtherBodyIndex :type Integer))
  (bind _mystep (`self.MyStep`))
  (bind _elevator (`self.Elevator`))
  (cast `/Game/Blueprints/BP_ThirdPersonCharacter` OtherActor)
  (if (== (`/Game/Blueprints/BP_Platform.currentFloor` _elevator) (`self.MyStep`))
    (`/Game/Blueprints/BP_Platform.MoveToFloor` _elevator (- _mystep 1) :!label _label)
    (elif (< (`/Game/Blueprints/BP_Platform.currentFloor` _elevator) (`self.MyStep`))
      (goto _label)
      (else
        (`/Game/Blueprints/BP_Platform.MoveToFloor` _elevator _mystep)))))

(fn `UserConstructionScript`)