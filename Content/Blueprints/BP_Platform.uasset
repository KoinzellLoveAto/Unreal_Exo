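; BP_Platform is a platform actor that moves up or down in steps along its own up vector when GoUp or GoDown is called.
; Both pass a direction to MoveToDirection, which sets a target one StepAmount from the current location, and record the state in IsUp.
; Tick eases the actor toward that target with a fixed-alpha lerp, without sweep, so the motion is frame-rate dependent.
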(event `self.ReceiveBeginPlay`
  (set `self.TargetPosition` (`self.K2_GetActorLocation`)))

(event `self.ReceiveTick`
  (params (DeltaSeconds :type "Float (single-precision)"))
  (`self.K2_SetActorLocation` (`KismetMathLibrary.VLerp` (`self.K2_GetActorLocation`) (`self.TargetPosition`) 0.05)))

(fn `GoDown`
  (`self.MoveToDirection` (* (`self.GetActorUpVector`) -1.0))
  (set `self.bIsUp` false))

(fn `GoUp`
  (`self.MoveToDirection` (`self.GetActorUpVector`))
  (set `self.bIsUp` true))

(fn `MoveToDirection`
  (params (Direction :type "Vector Structure"))
  (set `self.TargetPosition` (+ (* (`KismetMathLibrary.Normal` Direction) (`self.stepAmount`)) (`self.K2_GetActorLocation`))))

(fn `UserConstructionScript`)